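; BP_Webcam is an actor that shows a live webcam preview on a plane and takes captures on a key press.
; BeginPlay opens the camera through WebcamCapture and feeds its preview texture into a dynamic M_Webcam material on PlaneComp.
; Pressing F requests a capture from the component.
; Countdown, captured JPEG byte length and errors from its events are only printed to screen.
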(event `self.ReceiveBeginPlay`
  (`WebcamCapture.OpenCamera` (`self.WebcamCapture`))
  (`self.EnableInput` (`GameplayStatics.GetPlayerController` 0))
  (bind _returnvalue (`KismetMaterialLibrary.CreateDynamicMaterialInstance` "/Game/UI/RenderTexture/M_Webcam.M_Webcam"))
  (bind _output_get (set `self.DynMat` _returnvalue))
  (`MaterialInstanceDynamic.SetTextureParameterValue` _output_get "CamTex" (`WebcamCapture.GetPreviewTexture` (`self.WebcamCapture`)))
  (`PrimitiveComponent.SetMaterial` (`self.PlaneComp`) 0 (`self.DynMat`)))

(event `Key|F`
  (params (Key :type "Key Structure"))
  (:`Pressed`
    (`WebcamCapture.RequestCapture` (`self.WebcamCapture`))))

(event `self.WebcamCapture.OnFrameCaptured`
  (params (JpegBytes :type "Array of Byte (by ref)"))
  (`KismetSystemLibrary.PrintString` (`KismetStringLibrary.Concat_StrStr` "JEPG Bytes Length: " (`KismetStringLibrary.Conv_IntToString` (`KismetArrayLibrary.Array_Length` JpegBytes)))))

(event `self.WebcamCapture.OnCountdown`
  (params (RemainingSeconds :type "Float (single-precision)"))
  (`KismetSystemLibrary.PrintString` (`KismetStringLibrary.Concat_StrStr` "잔여 시간: " (`KismetStringLibrary.Conv_IntToString` (`KismetMathLibrary.FTrunc` RemainingSeconds)) "초")))

(event `self.WebcamCapture.OnCaptureError`
  (params (Error :type String))
  (`KismetSystemLibrary.PrintString` Error))

(fn `UserConstructionScript`)